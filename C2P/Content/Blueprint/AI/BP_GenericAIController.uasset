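; AI controller for generic enemies that runs BT_AI_Generic and feeds its blackboard from perception and death events.
; Sighting a Player-tagged actor sets it as target and switches state; lost sight or any other sense clears it, reports the last-seen location and triggers a ghost message.
; Tick continually writes spawn location, patrol-path flag and last sensed location.
; Death sets the dead state and forwards the message to the pawn.
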(event `/Game/Blueprint/AI/BPI_PatrolRouteInterface.HandleDeath`
  (params (`isDead?` :type Boolean))
  (bind _output_get (set `self.isDead?` `isDead?`))
  (`BlackboardComponent.SetValueAsEnum` (`AIBlueprintHelperLibrary.GetBlackboard` null) "currentState" 4)
  (message `/Game/Blueprint/AI/BPI_PatrolRouteInterface.HandleDeath` (`self.K2_GetPawn`) _output_get))

(event `self.ReceiveBeginPlay`
  (`self.RunBehaviorTree` "/Game/Blueprint/AI/BT_AI_Generic.BT_AI_Generic"))

(event `self.ReceiveTick`
  (params (DeltaSeconds :type "Float (single-precision)"))
  (`BlackboardComponent.SetValueAsVector` (`AIBlueprintHelperLibrary.GetBlackboard` null) "spawnLocation" (`self.SpawnLocation`))
  (`BlackboardComponent.SetValueAsBool` (`AIBlueprintHelperLibrary.GetBlackboard` null) "shouldPatrolOnPath?" (`self.shouldPatrolOnPath?`))
  (bind _info (`AIPerceptionComponent.GetActorsPerception` (`self.AIPerception`) (stale `self.AIPerception.OnTargetPerceptionUpdated` Actor)))
  (bind _output_get (set `self.playerLastSeenLocation` (`.StimulusLocation` (break `AIStimulus` (`|GetArrayItem` (`.LastSensedStimuli` (break `ActorPerceptionBlueprintInfo` _info)))))))
  (`BlackboardComponent.SetValueAsVector` (`AIBlueprintHelperLibrary.GetBlackboard` null) "targetActorLastSeenLocation" _output_get))

(event `self.AIPerception.OnTargetPerceptionUpdated`
  (params (Actor :type "Actor Object Reference") (Stimulus :type "AIStimulus Structure"))
  (bind (_age _expirationage _strength _stimuluslocation _receiverlocation _tag _bsuccessfullysensed) (break `AIStimulus` Stimulus))
  (if (not (`self.isDead?`))
    (if (`self.ActorHasTag` Actor "Player")
      (set `self.targetActor` Actor)
      (bind _returnvalue (`AIPerceptionSystem.GetSenseClassForStimulus` Stimulus))
      (if (== _returnvalue "/Script/AIModule.AISense_Sight")
        (if _bsuccessfullysensed
          (`BlackboardComponent.SetValueAsObject` (`AIBlueprintHelperLibrary.GetBlackboard` null) "targetActor" Actor)
          (set `self.playerLastSeenLocation` _stimuluslocation)
          (`BlackboardComponent.SetValueAsBool` (`AIBlueprintHelperLibrary.GetBlackboard` null) "canSeeTargetActor?" true)
          (`BlackboardComponent.SetValueAsEnum` (`AIBlueprintHelperLibrary.GetBlackboard` null) "currentState" 2)
          (else
            (`BlackboardComponent.SetValueAsObject` (`AIBlueprintHelperLibrary.GetBlackboard` null) "targetActor" null :!label _label)
            (`BlackboardComponent.SetValueAsVector` (`AIBlueprintHelperLibrary.GetBlackboard` null) "reportedLocation" (`self.playerLastSeenLocation`))
            (`BlackboardComponent.SetValueAsBool` (`AIBlueprintHelperLibrary.GetBlackboard` null) "canSeeTargetActor?" false)
            (message `/Game/Blueprint/Blueprint/BPI_SpawnGhost.SpawnGhost` (`self.targetActor`))
            (`KismetSystemLibrary.Delay` 0.1)
            (set `self.targetActor` null)))
        (else
          (goto _label))))
    (else
      (`BlackboardComponent.SetValueAsEnum` (`AIBlueprintHelperLibrary.GetBlackboard` null) "currentState" 4))))

(fn `GetPatrolRoute`
  (returns (PatrolRoute :type "/Game/Blueprint/Blueprint/BP_PatrolPath Object Reference"))
  (return (`self.PatrolRoute`)))

(fn `UserConstructionScript`)