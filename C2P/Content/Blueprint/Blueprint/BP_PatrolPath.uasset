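; BP_PatrolPath is a spline-based patrol route that supplies world-space waypoints from its PatrolPath spline.
; GetSplinePointAsWorldPosition returns the location of the spline point at the current PatrolIndex.
; IncrementPatrolRoute steps that index by Direction and flips Direction at the first and last points, so the route ping-pongs instead of looping.
; The index and direction are stored on the path itself.
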(event `IncrementPatrolRoute`
  (bind _output_get (set `self.patrolIndex` (+ (`self.patrolIndex`) (`self.direction`))))
  (if (== _output_get (- (`SplineComponent.GetNumberOfSplinePoints` (`self.patrolPath`)) 1))
    (set `self.direction` -1)
    (elif (== (`self.patrolIndex`) 0)
      (set `self.direction` 1))))

(fn `getSplinePointAsWorldPosition`
  (returns (Location :type "Vector Structure"))
  (return (`SplineComponent.GetLocationAtSplinePoint` (`self.patrolPath`) (`self.patrolIndex`) "World")))

(fn `UserConstructionScript`)