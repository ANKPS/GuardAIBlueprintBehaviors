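; BP_Ghost is a short-lived ghost actor with a skeletal mesh that fades out and destroys itself.
; Its delayed Tick resolves the player's BP_ThirdPersonCharacter as owner, then clears that character's ShouldSpawnGhost flag and applies a dynamic M_Ghost material to the mesh.
; A one-time FadeOut timeline drives material opacity, then hides the mesh, re-enables the owner's spawn flag and destroys the actor.
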(event `self.ReceiveBeginPlay`)

(event `self.ReceiveTick`
  (params (DeltaSeconds :type "Float (single-precision)"))
  (bind _owneractor (`self.ownerActor`))
  (`KismetSystemLibrary.Delay` 0.2)
  (`/Engine/EditorBlueprintResources/StandardMacros.IsValid` _owneractor
    (:`Is Valid`
      (set `/Game/ThirdPerson/Blueprints/BP_ThirdPersonCharacter.shouldSpawnGhost?` false _owneractor)
      (bind _returnvalue (`KismetMaterialLibrary.CreateDynamicMaterialInstance` "/Game/Blueprint/Material/M_Ghost.M_Ghost"))
      (bind _output_get (set `self.MID` _returnvalue))
      (`PrimitiveComponent.SetMaterial` (`self.SkeletalMesh`) 0 _output_get)
      (`PrimitiveComponent.SetMaterial` (`self.SkeletalMesh`) 1 _output_get)
      (`KismetSystemLibrary.Delay` 0.5)
      (`/Engine/EditorBlueprintResources/StandardMacros.DoOnce` false
        (:`Completed`
          (bind (_direction _fade_value) (`Timeline|FadeOut` :!via `PlayFromStart`)
            (:`Update`
              (`MaterialInstanceDynamic.SetScalarParameterValue` (`self.MID`) "Opacity" _fade_value))
            (:`Finished`
              (`SceneComponent.SetVisibility` (`self.SkeletalMesh`) false false)
              (`KismetSystemLibrary.Delay` 0.1)
              (set `/Game/ThirdPerson/Blueprints/BP_ThirdPersonCharacter.shouldSpawnGhost?` true (`self.ownerActor`))
              (`self.K2_DestroyActor`))))))
    (:`Is Not Valid`
      (bind _asbp_third_person_character (cast `/Game/ThirdPerson/Blueprints/BP_ThirdPersonCharacter` (`GameplayStatics.GetPlayerCharacter` 0)))
      (set `self.ownerActor` _asbp_third_person_character))))

(fn `UserConstructionScript`)