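; BP_Guard is an AI guard character that passes its patrol setup to its BP_GenericAIController and ragdolls on death.
; On BeginPlay it gives the controller its mesh location as the spawn point, plus the patrol route if valid.
; Tick copies the patrol-on-path flag to the controller every frame.
; HandleDeath sets mesh physics from the death flag and makes the capsule ignore a custom collision channel.
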(event `/Game/Blueprint/AI/BPI_PatrolRouteInterface.HandleDeath`
  (params (`isDead?` :type Boolean))
  (`PrimitiveComponent.SetSimulatePhysics` (`self.Mesh`) `isDead?`)
  (`PrimitiveComponent.SetCollisionResponseToChannel` (`self.CapsuleComponent`) "ECC_GameTraceChannel1" "ECR_Ignore"))

(event `self.ReceiveBeginPlay`
  (bind _patrol_route (`self.Patrol Route`))
  (bind _asbp_generic_aicontroller (cast `/Game/Blueprint/AI/BP_GenericAIController` (`self.GetController`)))
  (set `/Game/Blueprint/AI/BP_GenericAIController.SpawnLocation` (`SceneComponent.K2_GetComponentLocation` (`self.Mesh`)) _asbp_generic_aicontroller)
  (`/Engine/EditorBlueprintResources/StandardMacros.IsValid` _patrol_route
    (:`Is Valid`
      (set `/Game/Blueprint/AI/BP_GenericAIController.PatrolRoute` _patrol_route _asbp_generic_aicontroller))))

(event `self.ReceiveTick`
  (params (DeltaSeconds :type "Float (single-precision)"))
  (bind _asbp_generic_aicontroller (cast `/Game/Blueprint/AI/BP_GenericAIController` (`self.GetController`)))
  (set `/Game/Blueprint/AI/BP_GenericAIController.shouldPatrolOnPath?` (`self.shouldPatrolOnPath?`) _asbp_generic_aicontroller))

(fn `GetPatrolRoute`
  (returns (PatrolRoute :type "/Game/Blueprint/Blueprint/BP_PatrolPath Object Reference"))
  (return null))

(fn `UserConstructionScript`)